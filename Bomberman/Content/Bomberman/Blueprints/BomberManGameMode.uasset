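; Game mode for a two-player Bomberman match that runs the round timer and decides the winner or a draw.
; A Delay on Tick paces a once-per-second minutes/seconds countdown, which calls TimeOut at zero to show the draw menu.
; PlayerKilled awards the win to the other player and shows the winner menu; both endings pause the game.
; AddToPlayersArray stores bombers by index.
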(event Custom|TimeOut
  (Variables|Default|SetGameInProgress false)
  (Variables|Default|SetWinner "NewEnumerator2")
  (Game|SetGamePaused true)
  (bind _returnvalue (UserInterface|CreateWidget "/Game/Bomberman/Blueprints/DrawMenu.DrawMenu_C" (Game|GetPlayerController 0)))
  (UserInterface|Viewport|AddtoViewport _returnvalue 0))

(event Custom|AddToPlayersArray
  (params (Index :type Integer) (Bomber :type Bomberman%20Player%20Object%20Reference))
  (Utilities|Array|SetArrayElem (Variables|Default|GetPlayers) Index Bomber true))

(event Custom|PlayerKilled
  (params (PlayerType :type PlayerEnum%20Enum :default "NewEnumerator0"))
  (Variables|Default|SetGameInProgress false)
  (Game|SetGamePaused true)
  (if (Utilities|Enum|Equal(Enum) PlayerType "NewEnumerator0")
    (Variables|Default|SetWinner "NewEnumerator1")
    (else
      (Variables|Default|SetWinner "NewEnumerator0")))
  (bind _returnvalue (UserInterface|CreateWidget "/Game/Bomberman/Blueprints/PlayerWonMenu.PlayerWonMenu_C" (Game|GetPlayerController 0)))
  (UserInterface|Viewport|AddtoViewport _returnvalue 0))

(event EventBeginPlay)

(event EventTick
  (params (DeltaSeconds :type Float%20%28single-precision%29))
  (Utilities|FlowControl|Delay 1.0)
  (if (Variables|Default|GetGameInProgress)
    (Utilities|AnyTimeLeft
      (:True
        (if (== (Variables|Default|GetSecondsRemaining) 0)
          (Variables|Default|SetMinutesRemaining (- (Variables|Default|GetMinutesRemaining) 1))
          (Variables|Default|SetSecondsRemaining 59)
          (else
            (Variables|Default|SetSecondsRemaining (- (Variables|Default|GetSecondsRemaining) 1))
            (Utilities|AnyTimeLeft
              (:False
                (Variables|Default|SetGameInProgress false)
                (CallFunction|TimeOut)))))))))

(fn ConstructionScript)