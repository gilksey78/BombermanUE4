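; Bomberman player Blueprint that sets up each player's identity, bombs, score and death.
; On initialisation it picks player type and material from the controller ID and registers with BomberManGameMode, which is also notified on death.
; Spawned bombs receive their owner and radius upgrade, and the remote upgrade keeps a reference for manual detonation.
; Scoring triggers a temporary multiplier boost that steps down through delays.
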(event Custom|Die
  (bind _asbomber_man_game_mode (Utilities|Casting|CastToBomberManGameMode (Game|GetGameMode)))
  (Default|PlayerKilled _asbomber_man_game_mode (Variables|Default|GetPlayerType)))

(event Custom|AddToScore
  (params (ScoreToAdd :type Integer))
  (bind _output_get (Variables|Default|SetScore (+ (Variables|Default|GetScore) (* ScoreToAdd (Variables|Default|GetScoreMultiplier)))))
  (Development|PrintString (Utilities|String|ToString(Integer) _output_get))
  (if (not (Variables|Default|GetMultiplierActive))
    (Variables|Default|SetMultiplierActive true)
    (Variables|Default|SetScoreMultiplier 300)
    (Utilities|FlowControl|Delay 1.0)
    (Variables|Default|SetScoreMultiplier 200)
    (Utilities|FlowControl|Delay 1.0)
    (Variables|Default|SetScoreMultiplier 100)
    (Variables|Default|SetMultiplierActive false)))

(event EventBeginPlay)

(event Collision|EventActorBeginOverlap
  (params (OtherActor :type Actor%20Object%20Reference)))

(event EventTick
  (params (DeltaSeconds :type Float%20%28single-precision%29)))

(event EventRemoteDestroy
  (bind _remotebomb (Variables|Default|GetRemoteBomb))
  (if (Utilities|IsValid _remotebomb)
    (Default|BlowUp _remotebomb)))

(event EventSpawnBomb
  (params (upgradeActive :type Boolean))
  (bind _returnvalue (Game|SpawnActorfromClass "/Game/Bomberman/Blueprints/BP_Bomb.BP_Bomb_C" (Math|Conversions|ToTransform(Vector) (Transformation|GetActorLocation)) "Undefined" 0 0))
  (Variables|/Game/Bomberman/Blueprints/BP_Bomb.BP_Bomb_C|SetDropper _returnvalue self)
  (Variables|/Game/Bomberman/Blueprints/BP_Bomb.BP_Bomb_C|SetUpgradeActive _returnvalue (Variables|Default|GetbBombRadiusUpgradeActive))
  (if (Variables|Default|GetbRemoteBombUpgradeActive)
    (Variables|Default|SetRemoteBomb _returnvalue)))

(event EventPlayersInitialised
  (bind _controllerid (Variables|Default|GetControllerID))
  (if (== _controllerid 1)
    (Variables|Default|SetPlayerType "NewEnumerator1")
    (Rendering|Material|SetMaterial (Variables|Default|GetCube) 0 "/Game/Bomberman/Materials/M_P2.M_P2")
    (else
      (Variables|Default|SetPlayerType "NewEnumerator0")))
  (bind _asbomber_man_game_mode (Utilities|Casting|CastToBomberManGameMode (Game|GetGameMode)))
  (Default|AddtoPlayersArray _asbomber_man_game_mode _controllerid self))

(fn ConstructionScript)