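; Bomberman bomb actor that explodes after a short fuse, or a much longer one for remote bombs, and notifies its dropper.
; BlowUp line-traces in four grid directions through BlastTrace, adding a second segment per direction when upgraded, unless a wall blocks it.
; BlastTrace destroys crates for score, destroys pickups, kills players and chain-detonates other bombs.
; The scale timeline is unconnected and never runs.
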(event Custom|BlowUp
  (bind _returnvalue (Math|Vector|MakeVector 0.0 1e+02 0.0))
  (bind _returnvalue_2 (Transformation|GetActorLocation))
  (bind _returnvalue_3 (Transformation|GetActorLocation))
  (bind _returnvalue_4 (Transformation|GetActorLocation))
  (bind _returnvalue_5 (Transformation|GetActorLocation))
  (bind _returnvalue_6 (Math|Vector|MakeVector 1e+02 0.0 0.0))
  (bind _returnvalue_7 (Transformation|GetActorLocation))
  (bind _returnvalue_8 (Transformation|GetActorLocation))
  (bind _returnvalue_9 (Math|Vector|MakeVector 0.0 1e+02 0.0))
  (bind _returnvalue_10 (Transformation|GetActorLocation))
  (bind _returnvalue_11 (Transformation|GetActorLocation))
  (bind _returnvalue_12 (Math|Vector|MakeVector 1e+02 0.0 0.0))
  (bind _dropper (Variables|Default|GetDropper))
  (bind _dropper_2 (Variables|Default|GetDropper))
  (bind _returnvalue_13 (- _returnvalue_11 _returnvalue_12))
  (bind _returnvalue_14 (- _returnvalue_8 _returnvalue_9))
  (bind _returnvalue_15 (+ _returnvalue_10 _returnvalue_6))
  (bind _returnvalue_16 (+ _returnvalue_7 _returnvalue))
  (Class|BomberManCharacter|OnBombDestroy (Variables|Default|GetDropper))
  (Effects|SpawnEmitteratLocation "/Game/StarterContent/Particles/P_Explosion.P_Explosion" (Transformation|GetActorLocation))
  (Actor|DestroyActor)
  (if (Variables|Default|GetUpgradeActive)
    (Utilities|FlowControl|Sequence
      (:then_0
        (Development|PrintString "a" false)
        (Utilities|BlastTrace _returnvalue_10 _returnvalue_15 _dropper_2
          (:Out
            (Utilities|BlastTrace _returnvalue_15 (+ _returnvalue_15 _returnvalue_6) _dropper_2))))
      (:then_1
        (Development|PrintString "b" false)
        (Utilities|BlastTrace _returnvalue_11 _returnvalue_13 _dropper_2
          (:Out
            (Utilities|BlastTrace _returnvalue_13 (- _returnvalue_13 _returnvalue_12) _dropper_2))))
      (:then_2
        (Development|PrintString "c" false)
        (Utilities|BlastTrace _returnvalue_7 _returnvalue_16 _dropper_2
          (:Out
            (Utilities|BlastTrace _returnvalue_16 (+ _returnvalue_16 _returnvalue) _dropper_2))))
      (:then_3
        (Development|PrintString "d" false)
        (Utilities|BlastTrace _returnvalue_8 _returnvalue_14 _dropper_2
          (:Out
            (Utilities|BlastTrace _returnvalue_14 (- _returnvalue_14 _returnvalue_9) _dropper_2)))))
    (else
      (Development|PrintString "a" false)
      (Utilities|BlastTrace _returnvalue_2 (+ _returnvalue_2 (Math|Vector|MakeVector 1e+02 0.0 0.0)) _dropper
        (:Out
          _)
        (:HitWall
          _))
      (Development|PrintString "b" false)
      (Utilities|BlastTrace _returnvalue_3 (- _returnvalue_3 (Math|Vector|MakeVector 1e+02 0.0 0.0)) _dropper
        (:Out
          _)
        (:HitWall
          _))
      (Development|PrintString "c" false)
      (Utilities|BlastTrace _returnvalue_4 (+ _returnvalue_4 (Math|Vector|MakeVector 0.0 1e+02 0.0)) _dropper
        (:Out
          _)
        (:HitWall
          _))
      (Development|PrintString "d" false)
      (Utilities|BlastTrace _returnvalue_5 (- _returnvalue_5 (Math|Vector|MakeVector 0.0 1e+02 0.0)) _dropper))))

(event EventBeginPlay
  (if (Variables|Default|GetRemoteBomb)
    (Utilities|FlowControl|Delay 9e+01)
    (CallFunction|BlowUp)
    (else
      (Utilities|FlowControl|Delay 3.0)
      (CallFunction|BlowUp))))

(event Collision|EventActorBeginOverlap
  (params (OtherActor :type Actor%20Object%20Reference)))

(event EventTick
  (params (DeltaSeconds :type Float%20%28single-precision%29)))

(fn ConstructionScript)